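; BP_Thorns is a passive that reacts when its victim player takes damage by striking back at nearby enemies.
; Plugin binds Boom to the player's OnTakeAnyDamage event.
; Boom runs a small sphere overlap at the player's camera for BP_Base_Enemy pawns and sends each BI_Enemy implementer a zero-damage PunchMessage of type Disposable, regardless of the damage received or its source.
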(event `/Game/scripts/Core/BI_Passive.PlugIn`
  (add `Actor.OnTakeAnyDamage` (`self.VictimPlayer`) (delegate `Boom`)))

(event `Boom`
  (params (DamagedActor :type "Actor Object Reference") (Damage :type "Float (single-precision)") (DamageType :type "DamageType Object Reference") (InstigatedBy :type "Controller Object Reference") (DamageCauser :type "Actor Object Reference"))
  (bind _outactors (`KismetSystemLibrary.SphereOverlapActors` (`SceneComponent.K2_GetComponentLocation` (`MyCharacter.PlayerCamera` (`self.VictimPlayer`))) 32.0 (`|MakeArray` "ObjectTypeQuery3" :!type "EObjectTypeQuery Enum") "/Game/scripts/Enemies/BP_Base_Enemy.BP_Base_Enemy_C" (`|MakeArray` (`self.VictimPlayer`) :!type "Actor Object Reference")))
  (for _array_element _outactors
    (if (`KismetSystemLibrary.DoesImplementInterface` _array_element "/Game/scripts/Enemies/BI_Enemy.BI_Enemy_C")
      (message `/Game/scripts/Enemies/BI_Enemy.Punch` _array_element 0.0 "Disposable"))))

(fn `UserConstructionScript`
  (`parent.UserConstructionScript`))