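; BP_Shiza is a passive that afflicts its victim player with bouts of madness ("shiza").
; The Plugin event starts a looping timer with a random interval of roughly three seconds, picked once at setup.
; Each tick of that timer briefly flashes a random distressed Russian phrase through the GameState and makes VictimPlayer fire via Shoote.
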(event `/Game/scripts/Core/BI_Passive.PlugIn`
  (bind _returnvalue (`KismetSystemLibrary.K2_SetTimerDelegate` (delegate `Shiza`) (`KismetMathLibrary.RandomFloatInRange` 2.5 3.0) true))
  (set `self.ShizaTimer` _returnvalue))

(event `Shiza`
  (message `/Game/scripts/Core/BI_BaseGameState.Flash` (`GameplayStatics.GetGameState`) (`KismetArrayLibrary.Array_Random` (`|MakeArray` "ПОМОГИТЕ" "Я ХОЧУ ДОМОЙ" "Я НЕ ДОЛЖНА ПЕРЕРОДИТЬСЯ МАРИОНЕТКОЙ СНОВА" "МАМА ПРОСТИ МЕНЯ" "МНОГАБУКАВ" :!type "Text")) 0.05)
  (`/Game/scripts/Core/BP_TempCharacter.Shoote` (`self.VictimPlayer`)))

(fn `UserConstructionScript`
  (`parent.UserConstructionScript`))