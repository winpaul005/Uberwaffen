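; BP_Base_Enemy is a base enemy that chases the first DefaultPawn it finds and attacks it within AttackRange.
; Tick looks up the target and checks distance, moving toward its navmesh-projected location with AIMoveTo when out of range.
; In range, Attack runs behind a CanAttack flag with a one-second Delay cooldown, and currently only prints a damage message.
; The chase branch also sets a looping timer each Tick, with no event shown bound.
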(event `self.ReceiveBeginPlay`)

(event `self.ReceiveTick`
  (params (DeltaSeconds :type "Float (single-precision)"))
  (bind _returnvalue (`GameplayStatics.GetActorOfClass` "/Script/Engine.DefaultPawn"))
  (if (< (`self.GetDistanceTo` _returnvalue) (`self.AttackRange`))
    (if (`self.CanAttack`)
      (`self.Attack`)
      (set `self.CanAttack` false)
      (`KismetSystemLibrary.Delay` 1.0)
      (set `self.CanAttack` true))
    (else
      (`KismetSystemLibrary.K2_SetTimerDelegate` :`Time` 0.5 :`bLooping` true)
      (`|AIMoveTo` self (`NavigationSystemV1.K2_ProjectPointToNavigation` (`self.K2_GetActorLocation` _returnvalue)) null 150.0))))

(fn `Attack`
  (`KismetSystemLibrary.PrintString` "Damaged!"))

(fn `UserConstructionScript`)