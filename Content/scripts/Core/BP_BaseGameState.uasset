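; Game state hub for a level-based game, linking the player, main UI widget and jukebox while tracking level index, stat points and deaths.
; It relays weapon, ammo, passive and reload updates to the UI and applies passives and stat upgrades to the player.
; A filling stat meter awards points against a rising threshold.
; Stage and death events route to passive selection, intermission, death or end screens, and level changes reset the player.
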(event `self.ReceiveBeginPlay`
  (bind _returnvalue (`GameplayStatics.GetActorOfClass` "/Game/scripts/Core/BP_JukeBox.BP_JukeBox_C"))
  (bind _output_get (set `self.Jukeebox` _returnvalue))
  (`/Game/scripts/Core/BP_JukeBox.PlayCue` _returnvalue 1)
  (`/Game/scripts/Core/BP_JukeBox.PlayCue` _output_get 1))

(event `/Game/scripts/Core/BI_BaseGameState.SetUI`
  (params (UI :type "/Game/scripts/UI/BP_UI Object Reference"))
  (set `self.UI` UI))

(event `/Game/scripts/Core/BI_BaseGameState.UpdateWeapon`
  (params (Wepon :type "WeaponItem Structure"))
  (`/Game/scripts/UI/BP_UI.UpateWeapon` (`self.UI`) Wepon))

(event `/Game/scripts/Core/BI_BaseGameState.UpdateAmmo`
  (params (Cur :type Integer) (Max :type Integer))
  (`/Game/scripts/UI/BP_UI.UpdateAmmo` (`self.UI`) Cur Max))

(event `/Game/scripts/Core/BI_BaseGameState.UpdatePassives`
  (params (PassiveList :type "Array of Actor Object Reference (by ref)")))

(event `/Game/scripts/Core/BI_BaseGameState.AddPassive`
  (params (Passive :type "Actor Object Reference"))
  (`/Game/scripts/UI/BP_UI.AddPassive` (`self.UI`) Passive))

(event `/Game/scripts/Core/BI_BaseGameState.RemovePassive`
  (params (Idx :type Integer))
  (`PanelWidget.ClearChildren` (`/Game/scripts/UI/BP_UI.VerticalBox_0` (`self.UI`))))

(event `EnhancedInput|/Game/scripts/Core/IA_RevealPassives`
  (params (ActionValue :type Boolean) (ElapsedSeconds :type "Float (double-precision)") (TriggeredSeconds :type "Float (double-precision)") (InputAction :type "InputAction Object Reference" :default "/Game/scripts/Core/IA_RevealPassives.IA_RevealPassives")))

(event `/Game/scripts/Core/BI_BaseGameState.Flash`
  (params (Text :type Text) (Time :type "Float (double-precision)"))
  (`/Game/scripts/UI/BP_UI.Flash` (`self.UI`) Time Text))

(event `/Game/scripts/Core/BI_BaseGameState.StartCard`)

(event `/Game/scripts/Core/BI_BaseGameState.SetPlyr`
  (params (Plyr :type "/Game/scripts/Core/BP_TempCharacter Object Reference"))
  (set `self.Plyr` Plyr))

(event `/Game/scripts/Core/BI_BaseGameState.NextLevel`
  (params (Reset :type Boolean))
  (bind _ui (`self.UI`))
  (bind _jukeebox (`self.Jukeebox`))
  (bind _plyr (`self.Plyr`))
  ; До ресета добавить заглушку с выбором улучшения (тая что с дд)
  (if Reset
    (set `self.LevelIndex` 0)
    (set `self.StatPoints` 0)
    (`TextBlock.SetText` (`/Game/scripts/UI/BP_UI.StatPontMeter` _ui) "0")
    (`/Game/scripts/Core/BP_TempCharacter.ResetUITimer` _plyr)
    (`UserWidget.PlayAnimation` _ui (`/Game/scripts/UI/BP_UI.In` _ui) 0.0 1 "Forward" 1.0 false)
    (else
      (set `self.LevelIndex` (+ (`self.LevelIndex`) 1))))
  (`/Game/scripts/Core/BP_TempCharacter.Resetto` _plyr)
  (if (and (== (`/Game/scripts/Core/BP_JukeBox.currentCue` _jukeebox) 0) Reset)
    (`/Game/scripts/Core/BP_JukeBox.PlayCue` _jukeebox 1)))

(event `/Game/scripts/Core/BI_BaseGameState.PassStage`
  (params (IsDed :type Boolean))
  (bind _statpoints (`self.StatPoints`))
  (if (< (`self.LevelIndex`) (`self.TotalLevels`))
    (if IsDed
      (if (> _statpoints 0)
        (`/Game/scripts/UI/BP_UI.FadeToPassives` (`self.UI`) _statpoints IsDed :!label _label)
        (else
          (`self.PlayDeadIntermission`)))
      (else
        (goto _label)))
    (else
      (bind _returnvalue (`|CreateWidget` "/Game/scripts/UI/BP_End.BP_End_C" (`GameplayStatics.GetPlayerController` 0)))
      (`UserWidget.AddToViewport` _returnvalue 0))))

(event `/Game/scripts/Core/BI_BaseGameState.AttachPassive`
  (params (Name :type Name))
  (`/Game/scripts/Core/BP_TempCharacter.AddPassive` (`self.Plyr`) Name))

(event `/Game/scripts/Core/BI_BaseGameState.AddStatsMeter`
  (params (Delta :type "Float (double-precision)"))
  (bind _output_get (set `self.StatMeter` (+ (`self.StatMeter`) Delta)))
  (`KismetSystemLibrary.PrintText` (`|FormatText` "Addign stats: \n{X} \n" _output_get))
  (`self.AddStatPoint` (`self.StatMeter`)))

(event `/Game/scripts/Core/BI_BaseGameState.PlayIntermission`
  (params (`Intermission Instance` :type Name))
  (bind _returnvalue (`|CreateWidget` "/Game/scripts/UI/BP_Intermission.BP_Intermission_C" (`GameplayStatics.GetPlayerController` 0)))
  (bind _returnvalue_2 (`|GetDataTableRow` "/Game/scripts/Core/DT_IntermissionScenes.DT_IntermissionScenes" "a")
    (:`then`
      (`/Game/scripts/UI/BP_Intermission.Start` _returnvalue (`.Cards_3_B3CC296F4F2DF10BBA4B028018B8D73F` (break `/Game/scripts/Core/ST_IntermissionSt` _returnvalue_2))))
    (:`RowNotFound`
      (`/Game/scripts/UI/BP_Intermission.Intermission` _returnvalue)))
  (`UserWidget.AddToViewport` _returnvalue 0))

(event `/Game/scripts/Core/BI_BaseGameState.ItsOver`
  (`/Game/scripts/Core/BP_JukeBox.PlayCue` (`self.Jukeebox`) 0)
  (bind _returnvalue (`|CreateWidget` "/Game/scripts/UI/BP_DedScreen.BP_DedScreen_C" (`GameplayStatics.GetPlayerController` 0)))
  (`UserWidget.AddToViewport` _returnvalue 0))

(event `/Game/scripts/Core/BI_BaseGameState.PlayDeadIntermission`
  (bind _outactors (`GameplayStatics.GetAllActorsWithInterface` "/Game/scripts/Enemies/BI_Enemy.BI_Enemy_C"))
  (for _array_element _outactors
    (`self.K2_DestroyActor` _array_element))
  (`/Game/scripts/Core/BP_JukeBox.PlayCue` (`self.Jukeebox`) 0)
  (bind _returnvalue (`|CreateWidget` "/Game/scripts/UI/BP_Intermission.BP_Intermission_C" (`GameplayStatics.GetPlayerController` 0) true))
  (`/Game/scripts/UI/BP_Intermission.Intermission` _returnvalue)
  (`UserWidget.AddToViewport` _returnvalue 0))

(event `/Game/scripts/Core/BI_BaseGameState.AddPlyrStatPont`
  (params (StatID :type Byte))
  (bind _plyr (`self.Plyr`))
  (bind (_currentstats_speed _currentstats_ranged _currentstats_health) (break `/Game/scripts/Core/ST_Stats` (`/Game/scripts/Core/BP_TempCharacter.CurrentStats` _plyr)))
  (set `/Game/scripts/Core/BP_TempCharacter.CurrentStats` (make `/Game/scripts/Core/ST_Stats` (+ _currentstats_speed (* 1 (`KismetMathLibrary.Conv_BoolToInt` (== StatID 0)))) (+ _currentstats_ranged (* 1 (`KismetMathLibrary.Conv_BoolToInt` (== StatID 1)))) (+ _currentstats_health (* 1 (`KismetMathLibrary.Conv_BoolToInt` (== StatID 2))))) _plyr))

(event `/Game/scripts/Core/BI_BaseGameState.SetIsReloading`
  (params (ISRealoading :type Boolean))
  (`/Game/scripts/UI/BP_UI.Reloj` (`self.UI`) ISRealoading))

(event `/Game/scripts/Core/BI_BaseGameState.AddDeathCount`
  (set `self.TotalDeaths` (+ (`self.TotalDeaths`) 1)))

(fn `AddStatPoint`
  (params (StatPoints :type "Float (double-precision)"))
  (if (>= (/ StatPoints (`self.LevelUppe`)) 1.0)
    (set `self.StatMeter` 0.0)
    (set `self.LevelUppe` (+ (`self.LevelUppe`) 1))
    (bind _output_get (set `self.StatPoints` (+ (`self.StatPoints`) 1)))
    (`/Game/scripts/UI/BP_UI.UpdateStatPonts` (`self.UI`) _output_get)
    (`KismetSystemLibrary.PrintText` (`|FormatText` "CurrentStatsPoints: \n{X}" (`self.LevelUppe`)))))

(fn `GetGaymLevelle`
  (returns (NewParam :type Integer))
  (return (`self.LevelUppe`)))

(fn `GetHasDiedTooMuch`
  (returns (NewParam :type Boolean))
  (return (> (`self.TotalDeaths`) 7)))

(fn `GetIsDed`
  (returns (Ded :type Boolean))
  (return (`/Game/scripts/Core/BP_TempCharacter.IsDead` (`self.Plyr`))))

(fn `GetLevelIndex`
  (returns (Index :type Integer))
  (return (`self.LevelIndex`)))

(fn `GetMaxLevels`
  (returns (MaxLevel :type Integer))
  (return (`self.TotalLevels`)))

(fn `GetPlayerStats`
  (returns (stats :type "/Game/scripts/Core/ST_Stats Structure"))
  (return (`/Game/scripts/Core/BP_TempCharacter.CurrentStats` (`self.Plyr`))))

(fn `GetPlyrHealth`
  (returns (Healthg :type "Float (double-precision)") (maxHealth :type "Float (double-precision)"))
  (bind _plyr (`self.Plyr`))
  (return (`/Game/scripts/Core/BP_TempCharacter.Health` _plyr) (`/Game/scripts/Core/BP_TempCharacter.MaxHealth` _plyr)))

(fn `GetStatoMeter`
  (returns (NewParam :type "Float (double-precision)"))
  (return (`self.StatMeter`)))

(fn `GetStatPonts`
  (returns (statpoints :type Integer))
  (return (`self.StatPoints`)))

(fn `UserConstructionScript`)