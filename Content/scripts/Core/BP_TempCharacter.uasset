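; First-person player character for a shooter, handling weapons, health, passives, death and respawn.
; Data table weapons fill a bag; fire-mode logic drives shots as melee or ranged traces or RPG projectiles, with ammo, reload and switching.
; Passives spawn as plug-in actors from a data table and are destroyed on death.
; HUD updates go through GameState messages and a material parameter collection, while Resetto applies stats, revives and starts the level spawner.
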(event `self.ReceiveBeginPlay`
  (`self.ResetUITimer`)
  (message `/Game/scripts/Core/BI_BaseGameState.SetPlyr` (`GameplayStatics.GetGameState`) self)
  (set `self.Spawnpoint` (`self.K2_GetActorLocation`))
  (`EnhancedInputSubsystemInterface.AddMappingContext` (pcsubsystem `EnhancedInputLocalPlayerSubsystem` (`GameplayStatics.GetPlayerController` 0)) "/Game/scripts/Core/IMC_TMP.IMC_TMP" 0 (struct))
  ; Заглушки, убрать при билде
  (bind _returnvalue (`|GetDataTableRow` "/Game/Weapons.Weapons" "Shard")
    (:`then`
      (`self.AddWeaponToBag` _returnvalue)
      (bind _returnvalue_2 (`|GetDataTableRow` "/Game/Weapons.Weapons" "KA420")
        (:`then`
          (`self.AddWeaponToBag` _returnvalue_2)
          (for _array_element (`self.StarterPassives`)
            (`self.AddPassive` _array_element))
          (`self.Resetto`))))))

(event `EnhancedInput|/Game/scripts/Core/IA_Switch`
  (params (ActionValue :type "Float (double-precision)") (ElapsedSeconds :type "Float (double-precision)") (TriggeredSeconds :type "Float (double-precision)") (InputAction :type "InputAction Object Reference" :default "/Game/scripts/Core/IA_Switch.IA_Switch"))
  (:`Started`
    (if (< ActionValue 0.0)
      (`KismetSystemLibrary.PrintString` "Ping!")
      (`self.SwitchNextWep` true)
      (else
        (`KismetSystemLibrary.PrintString` "Pong!")
        (`self.SwitchNextWep` false)))))

(event `self.ReceiveTick`
  (params (DeltaSeconds :type "Float (single-precision)"))
  (bind _returnvalue (- (`self.DisortionTimer`) DeltaSeconds))
  (`self.CameraBobbing`)
  (if (> _returnvalue 0.0)
    (bind _output_get (set `self.DisortionTimer` _returnvalue))
    (`KismetMaterialLibrary.SetScalarParameterValue` "/Game/PlayerParams.PlayerParams" "Tymer" _output_get)))

(event `EnhancedInput|/Game/scripts/Core/IA_Shoot`
  (params (ActionValue :type Boolean) (ElapsedSeconds :type "Float (double-precision)") (TriggeredSeconds :type "Float (double-precision)") (InputAction :type "InputAction Object Reference" :default "/Game/scripts/Core/IA_Shoot.IA_Shoot"))
  (:`Triggered`
    (`self.ProcessShot` :!label _label))
  (:`Started`
    (goto _label :!via `Click`))
  (:`Completed`
    (`self.ShootEvent` true)
    (goto _label :!via `Release`)))

(event `Reload`
  (params (ReloadTimer :type "Float (double-precision)"))
  (bind _output (`|GetArrayItem` (`self.WeaponBag`) (`self.CurrentWeapom`)))
  (bind (_itemname _itemdescription _itemimage _viewportmesh _damagepattern _weapontype _maxammo _maxclipammo _clipammo _currentammo) (break `WeaponItem` _output))
  (if (not (`self.isRelaoding`))
    (`GameplayStatics.PlaySound2D` "/Game/audio/ReloadCue.ReloadCue" 1.0 1.0 0.0 null null)
    (`self.ReloadWeap`)
    (bind _output_get (set `self.isRelaoding` true))
    (message `/Game/scripts/Core/BI_BaseGameState.SetIsReloading` (`GameplayStatics.GetGameState`) _output_get)
    (`KismetSystemLibrary.Delay` ReloadTimer)
    (if (`self.isRelaoding`)
      (setmembers `WeaponItem` :`StructRef` _output :`clipAmmo` (`KismetMathLibrary.Clamp` _maxclipammo 0 _currentammo) :`currentAmmo` (`KismetMathLibrary.Clamp` (- _currentammo _maxclipammo) 0 _maxammo))
      (`self.UpdateVisuals` true)
      (message `/Game/scripts/Core/BI_BaseGameState.SetIsReloading` (`GameplayStatics.GetGameState`) false)
      (set `self.isRelaoding` false))))

(event `self.ReceiveAnyDamage`
  (params (Damage :type "Float (single-precision)") (DamageType :type "DamageType Object Reference") (InstigatedBy :type "Controller Object Reference") (DamageCauser :type "Actor Object Reference"))
  (`self.Punch` Damage))

(event `self.ReceiveRadialDamage`
  (params (DamageReceived :type "Float (single-precision)") (DamageType :type "DamageType Object Reference") (Origin :type "Vector Structure") (HitInfo :type "HitResult Structure (by ref)") (InstigatedBy :type "Controller Object Reference") (DamageCauser :type "Actor Object Reference"))
  (`self.Punch` DamageReceived))

(fn `AddAmmo`
  (bind _weaponbag (`self.WeaponBag`))
  (for (_array_element _array_index) _weaponbag
    (bind (_itemname _itemdescription _itemimage _viewportmesh _damagepattern _weapontype _maxammo _maxclipammo _clipammo _currentammo) (break `WeaponItem` _array_element))
    (bind _structout (setmembers `WeaponItem` :`StructRef` _array_element :`currentAmmo` (`KismetMathLibrary.Clamp` (+ _currentammo 3) 0 _maxammo)))
    (`KismetArrayLibrary.Array_Set` _weaponbag _array_index _structout))
  (`self.UpdateVisuals` true))

(fn `AddGimmmickWeapon`
  (bind _gimmickweaponidx (`self.GimmickWeaponIdx`))
  (bind _returnvalue (`|GetDataTableRow` "/Game/Weapons.Weapons" (`KismetArrayLibrary.Array_Random` (`|MakeArray` "M82" "RPG" :!type "Name")))
    (:`then`
      (if (>= _gimmickweaponidx 0)
        (`KismetArrayLibrary.Array_Remove` (`self.WeaponBag`) _gimmickweaponidx))
      (bind _index (`self.AddWeaponToBag` _returnvalue))
      (set `self.GimmickWeaponIdx` _index))))

(fn `AddPassive`
  (params (RowName :type Name))
  (bind _returnvalue (`|GetDataTableRow` "/Game/scripts/Passive/DT_Passives.DT_Passives" RowName)
    (:`then`
      (bind _returnvalue_2 (`KismetSystemLibrary.LoadClassAsset_Blocking` (`.Class_10_395BBDCE45BEF4F469E77789311E4A68` (break `/Game/scripts/Passive/ST_Passive` _returnvalue))))
      (bind _asactor (castclass `Actor` _returnvalue_2))
      (bind _returnvalue_3 (`|SpawnActorFromClass` _asactor (`self.GetTransform`) "Undefined" "MultiplyWithRoot" null null))
      (message `/Game/scripts/Core/BI_Passive.Setup` _returnvalue_3 _returnvalue self)
      (message `/Game/scripts/Core/BI_Passive.PlugIn` _returnvalue_3) ; Do whatever the f passive is supposed to
      (`KismetArrayLibrary.Array_Add` (`self.ActivePassives`) _returnvalue_3)
      (`KismetSystemLibrary.PrintString` "Passive spawned")
      (message `/Game/scripts/Core/BI_BaseGameState.AddPassive` (`GameplayStatics.GetGameState`) _returnvalue_3))))

(fn `AddWeaponToBag`
  (params (NewItem :type "WeaponItem Structure (by ref)"))
  (returns (Index :type Integer))
  (bind (_itemname _itemdescription _itemimage _viewportmesh _damagepattern _weapontype _maxammo _maxclipammo) (break `WeaponItem` NewItem))
  (for _array_element (`self.WeaponBag`)
    (if (`KismetStringLibrary.EqualEqual_StrStr` (`.ItemName` (break `WeaponItem` _array_element)) _itemname)
      (`KismetSystemLibrary.PrintString` "WEAPON ALREADY EXISTS!!" true true (struct :`R` 1.0 :`G` 0.093923 :`A` 1.0))
      (`self.AddAmmo`)
      (return -1)))
  (bind _structout (setmembers `WeaponItem` :`StructRef` NewItem :`clipAmmo` _maxclipammo :`currentAmmo` 0))
  (bind _returnvalue (`KismetArrayLibrary.Array_Add` (`self.WeaponBag`) _structout))
  (set `self.CurrentWeapom` _returnvalue)
  (`self.UpdateVisuals` false)
  (return _returnvalue))

(fn `CameraBobbing`
  (if (and (> (`KismetMathLibrary.VSize` (`self.GetVelocity`)) 10.0) (`self.CanJump`))
    (`PlayerController.ClientStartCameraShake` :`self` (`GameplayStatics.GetPlayerController` 0) :`Shake` "/Game/scripts/Camera/RunCameraShake.RunCameraShake_C")))

(fn `Heal`
  (params (Factor :type "Float (double-precision)"))
  (bind _output_get (set `self.Health` (`KismetMathLibrary.FClamp` (+ (`self.Health`) Factor) 0.0 (`self.MaxHealth`))))
  (`KismetMaterialLibrary.SetScalarParameterValue` "/Game/PlayerParams.PlayerParams" "Health" (`KismetMathLibrary.FClamp` (/ _output_get (`self.MaxHealth`)))))

(fn `Punch`
  (params (Vasl :type "Float (double-precision)"))
  (bind _activepassives (`self.ActivePassives`))
  (bind _returnvalue (- (`self.Health`) Vasl))
  (if (`self.IsDead`)
    _
    (elif (<= _returnvalue 0.0)
      (set `self.IsDead` true)
      (for _array_element _activepassives
        (`self.K2_DestroyActor` _array_element)
        (message `/Game/scripts/Core/BI_BaseGameState.RemovePassive` (`GameplayStatics.GetGameState`) 0))
      (`KismetArrayLibrary.Array_Clear` _activepassives)
      (message `/Game/scripts/Core/BI_BaseGameState.ItsOver` (`GameplayStatics.GetGameState`))
      (else
        (bind _output_get (set `self.Health` _returnvalue))
        (`KismetMaterialLibrary.SetScalarParameterValue` "/Game/PlayerParams.PlayerParams" "Health" (`KismetMathLibrary.FClamp` (/ _output_get (`self.MaxHealth`))))))))

(fn `Resetto`
  (bind _returnvalue (`GameplayStatics.GetPlayerController` 0))
  (bind _weaponbag (`self.WeaponBag`))
  (bind (_speed _ranged _health) (break `/Game/scripts/Core/ST_Stats` (`self.CurrentStats`)))
  (`WidgetBlueprintLibrary.SetInputMode_GameOnly` _returnvalue)
  (set `PlayerController.bShowMouseCursor` false _returnvalue)
  (set `CharacterMovementComponent.MaxWalkSpeed` (+ 800.0 (* _speed 10)) (`self.CharacterMovement`))
  (set `self.MaxHealth` (+ 100.0 (* _health 10)))
  (if (`self.IsDead`)
    (set `self.IsDead` false)
    (`self.K2_SetActorLocation` (`self.Spawnpoint`) false true)
    (`KismetMaterialLibrary.SetScalarParameterValue` "/Game/PlayerParams.PlayerParams" "Health" 1.0)
    (set `self.Health` (`self.MaxHealth`))
    (set `self.CurrentWeapom` 0)
    (for (_array_element _array_index) _weaponbag
      (bind _structout (setmembers `WeaponItem` :`StructRef` _array_element :`clipAmmo` (`.MaxClipAmmo` (break `WeaponItem` _array_element))))
      (`KismetArrayLibrary.Array_Set` _weaponbag _array_index _structout)))
  (`self.UpdateVisuals` false)
  (bind _returnvalue_2 (`GameplayStatics.GetActorOfClass` "/Game/scripts/Core/BP_Spawner.BP_Spawner_C"))
  (bind _index (message `/Game/scripts/Core/BI_BaseGameState.GetLevelIndex` (`GameplayStatics.GetGameState`)))
  (`/Game/scripts/Core/BP_Spawner.Begin` _returnvalue_2 _index))

(fn `ResetUITimer`
  (set `self.DisortionTimer` 2.0))

(fn `Shoote`
  (bind _rpgpoint (`self.RPGpoint`))
  (bind _playercamera (`self.PlayerCamera`))
  (bind _returnvalue (`SceneComponent.K2_GetComponentLocation` _playercamera))
  (bind _returnvalue_2 (`SceneComponent.GetForwardVector` _playercamera))
  (bind (_returnvalue_location _returnvalue_rotation _returnvalue_scale) (`KismetMathLibrary.BreakTransform` (`SceneComponent.K2_GetComponentToWorld` _rpgpoint)))
  (bind _output (`|GetArrayItem` (`self.WeaponBag`) (`self.CurrentWeapom`)))
  (bind (_itemname _itemdescription _itemimage _viewportmesh _damagepattern _weapontype _maxammo _maxclipammo _clipammo _currentammo _pewsound _shootcooldown _shootwarmup _damagefactor) (break `WeaponItem` _output))
  (bind _returnvalue_3 (> _clipammo 0))
  (if (`self.IsDead`)
    _
    (elif (or _returnvalue_3 (`|EnumEquality` _weapontype "Melee"))
      (setmembers `WeaponItem` :`StructRef` _output :`clipAmmo` (`KismetMathLibrary.Clamp` (- _clipammo 1) 0 _maxclipammo))
      (switch `EWeaponType` _weapontype
        (:`Melee`
          (bind _outhit (`KismetSystemLibrary.LineTraceSingle` _returnvalue (+ (* _returnvalue_2 200.0) _returnvalue) "TraceTypeQuery1"))
          (`KismetSystemLibrary.PrintString` "Damage Short"))
        (:`Ranged`
          ; здесь типо рейкаст от камеры (но она должна быть для начала, а для нее должен быть контролер)
          (bind _outhit_2 (`KismetSystemLibrary.LineTraceSingle` _returnvalue (+ (* _returnvalue_2 999999.0) _returnvalue) "TraceTypeQuery1")))
        (:`Disposable`
          (`|SpawnActorFromClass` "/Game/scripts/Core/BR_RPGProjectile.BR_RPGProjectile_C" (`KismetMathLibrary.MakeTransform` _returnvalue_location _returnvalue_rotation _returnvalue_scale) "Undefined" "MultiplyWithRoot" null (`SceneComponent.GetForwardVector` _rpgpoint) 90.0 null)))
      (`self.UpdateVisuals` true)
      (`self.ShootEvent` false)
      (bind (_bblockinghit _binitialoverlap _time _distance _location _impactpoint _normal _impactnormal _physmat _hitactor) (`GameplayStatics.BreakHitResult` (select `EWeaponType` _weapontype :`Melee` _outhit :`Ranged` _outhit_2)))
      (bind _returnvalue_4 (`GameplayStatics.SpawnDecalAtLocation` "/Game/MT_Bullet.MT_Bullet" (3.0 3.0 3.0) _impactpoint (`KismetMathLibrary.MakeRotFromX` _impactpoint) 4.0))
      (`GameplayStatics.PlaySound2D` _pewsound 1.0 1.0 0.0 null null)
      (`KismetSystemLibrary.PrintText` (`KismetTextLibrary.Conv_ObjectToText` (`ActorComponent.GetOwner` _returnvalue_4)))
      (if (`KismetSystemLibrary.DoesImplementInterface` _hitactor "/Game/scripts/Enemies/BI_Enemy.BI_Enemy_C")
        (message `/Game/scripts/Enemies/BI_Enemy.Punch` _hitactor (* (* (`.Ranged_10_B3092E5945EC1AE0DFF0BE94E386B01C` (break `/Game/scripts/Core/ST_Stats` (`self.CurrentStats`))) 0.4) _damagefactor) _normal "Melee"))
      (elif (and (or _returnvalue_3 (> _currentammo 0)) (not (`self.isRelaoding`)))
        (`self.ShootEvent` true)
        (`self.Reload` 1.5)
        (else
          (`self.ShootEvent` true))))))

(fn `SwitchNextWep`
  (params (IsReverse :type Boolean))
  (bind _currentweapom (`self.CurrentWeapom`))
  (bind _returnvalue (`KismetArrayLibrary.Array_Length` (`self.WeaponBag`)))
  (bind _returnvalue_2 (- _currentweapom 1))
  (bind _returnvalue_3 (+ _currentweapom 1))
  (if (not (`self.isRelaoding`))
    (if IsReverse
      (set `self.CurrentWeapom` (`KismetMathLibrary.SelectInt` (- _returnvalue 1) _returnvalue_2 (< _returnvalue_2 0)))
      (else
        (set `self.CurrentWeapom` (`KismetMathLibrary.SelectInt` 0 _returnvalue_3 (>= _returnvalue_3 _returnvalue)))))
    (if (`self.isRelaoding`)
      (set `self.isRelaoding` false)
      (message `/Game/scripts/Core/BI_BaseGameState.SetIsReloading` (`GameplayStatics.GetGameState`) false))
    (`self.UpdateVisuals` false)))

(fn `UpdateVisuals`
  (params (IsAmmo :type Boolean))
  (bind _returnvalue (`GameplayStatics.GetGameState`))
  (bind _output (`|GetArrayItem` (`self.WeaponBag`) (`self.CurrentWeapom`)))
  (bind (_itemname _itemdescription _itemimage _viewportmesh _damagepattern _weapontype _maxammo _maxclipammo _clipammo _currentammo) (break `WeaponItem` _output))
  (if IsAmmo
    (message `/Game/scripts/Core/BI_BaseGameState.UpdateAmmo` _returnvalue _clipammo _currentammo)
    (else
      (message `/Game/scripts/Core/BI_BaseGameState.UpdateWeapon` _returnvalue _output)
      (`SkeletalMeshComponent.SetSkeletalMeshAsset` (`self.Weapon`) _viewportmesh)
      (`self.SwitchWeaponAnim` _weapontype)
      (message `/Game/scripts/Core/BI_BaseGameState.UpdatePassives` _returnvalue (`self.ActivePassives`)))))

(fn `UserConstructionScript`)