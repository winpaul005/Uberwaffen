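; Wave spawner that releases delayed hordes of enemies at three random spawn points and passes the stage once all waves clear.
; Begin sets the wave count from the stage, then SpawnHalfWave picks randomly from DT_Enemies rows whose difficulty fits wave progress and level index.
; Tracked enemies leaving the Checker volume advance waves unless the game state reports death.
; The separate death event only untracks actors and prints when none remain.
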(event `self.ReceiveBeginPlay`)

(event `SpawnHalfWave`
  (if (> (`self.TotalWaves`) 0)
    (bind _outrownames (`DataTableFunctionLibrary.GetDataTableRowNames` "/Game/scripts/Core/DT_Enemies.DT_Enemies"))
    (bind _index (message `/Game/scripts/Core/BI_BaseGameState.GetLevelIndex` (`GameplayStatics.GetGameState`)))
    (for _array_element _outrownames
      (bind _returnvalue (`|GetDataTableRow` "/Game/scripts/Core/DT_Enemies.DT_Enemies" _array_element)
        (:`then`
          (if (<= (`.Difficulty_12_9B55A22A475246257E72D3830BDE2618` (break `/Game/scripts/Core/ST_Enemigo` _returnvalue)) (- (+ (`self.MaxWave`) _index) (`self.TotalWaves`)))
            (`KismetArrayLibrary.Array_Add` (`self.TotalAvailibleeEnemies`) _array_element)))))
    (`self.ForWithDelay` 0 (- (+ (`self.MaxEnemiesPerHalfWave`) _index) 1) (`self.HordeSpawnCooldown`)
      (:`LoopBody`
        (bind _returnvalue_2 (`|GetDataTableRow` "/Game/scripts/Core/DT_Enemies.DT_Enemies" (`KismetArrayLibrary.Array_Random` (`self.TotalAvailibleeEnemies`)))
          (:`then`
            (bind _returnvalue_3 (`KismetSystemLibrary.LoadClassAsset_Blocking` (`.Class_9_ACFB1D6A4FB9270DBCB70FBC4ADC04FC` (break `/Game/scripts/Core/ST_Enemigo` _returnvalue_2))))
            (bind _asactor (castclass `Actor` _returnvalue_3))
            (bind _returnvalue_4 (`|SpawnActorFromClass` _asactor (`SceneComponent.K2_GetComponentToWorld` (`KismetArrayLibrary.Array_Random` (`|MakeArray` (`self.S1`) (`self.S2`) (`self.S3`)))) "Undefined" "MultiplyWithRoot" null null))
            (`KismetArrayLibrary.Array_Add` (`self.SpawnedActors`) _returnvalue_4)))))))

(event `ReceveDesu_Event`
  (params (Actor :type "Actor Object Reference"))
  (`KismetArrayLibrary.Array_RemoveItem` (`self.SpawnedActors`) Actor)
  (if (<= (`KismetArrayLibrary.Array_Length` (`self.SpawnedActors`)) 0)
    (`KismetSystemLibrary.PrintString` "PASS!" true true (struct :`G` 1.0 :`B` 0.382096 :`A` 1.0))))

(event `self.Checker.OnComponentEndOverlap`
  (params (OverlappedComponent :type "PrimitiveComponent Object Reference") (OtherActor :type "Actor Object Reference") (OtherComp :type "PrimitiveComponent Object Reference") (OtherBodyIndex :type Integer))
  (bind _spawnedactors (`self.SpawnedActors`))
  (bind _returnvalue (- (`self.TotalWaves`) 1))
  (`KismetSystemLibrary.PrintString` "OUT!" true true (struct :`R` 1.0 :`G` 0.083057 :`A` 1.0))
  (if (>= (`KismetArrayLibrary.Array_Find` _spawnedactors OtherActor) 0)
    (`KismetArrayLibrary.Array_RemoveItem` _spawnedactors OtherActor)
    (bind _ded (message `/Game/scripts/Core/BI_BaseGameState.GetIsDed` (`GameplayStatics.GetGameState`)))
    (if (and (<= (`KismetArrayLibrary.Array_Length` (`self.SpawnedActors`)) 0) (not _ded))
      (if (<= _returnvalue 0)
        (message `/Game/scripts/Core/BI_BaseGameState.PassStage` (`GameplayStatics.GetGameState`) false)
        (else
          (set `self.TotalWaves` _returnvalue)
          (`self.SpawnHalfWave`))))))

(fn `Begin`
  (params (Stage :type Integer))
  (set `self.TotalWaves` (+ (`self.MaxWave`) Stage))
  (`self.SpawnHalfWave`))

(fn `UserConstructionScript`)