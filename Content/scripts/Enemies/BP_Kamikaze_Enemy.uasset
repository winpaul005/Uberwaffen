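; Kamikaze enemy that chases the player character (MyCharacter) and blows itself up when close.
; Every Tick it compares its distance to the player against ExplosionRange, moving via AIMoveTo toward the player's navmesh-projected location while out of range.
; Inside range, Explode applies full radial damage, spawns a particle effect and destroys the actor.
; The chase branch also sets a looping timer every Tick, with no event shown bound.
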(event `self.ReceiveBeginPlay`)

(event `self.ReceiveTick`
  (params (DeltaSeconds :type "Float (single-precision)"))
  (bind _returnvalue (`GameplayStatics.GetActorOfClass` "/Script/Uberwaffen.MyCharacter"))
  (if (< (`self.GetDistanceTo` _returnvalue) (`self.explosionRange`))
    (`self.Explode`)
    (else
      (`KismetSystemLibrary.K2_SetTimerDelegate` "" 0.5 true)
      (`|AIMoveTo` self (`NavigationSystemV1.K2_ProjectPointToNavigation` (`self.K2_GetActorLocation` _returnvalue)) null 150.0))))

(fn `Explode`
  (bind _returnvalue (`self.K2_GetActorLocation`))
  (`GameplayStatics.ApplyRadialDamage` :`BaseDamage` 50.0 :`Origin` _returnvalue :`DamageRadius` 300.0 :`DamageCauser` null :`InstigatedByController` null :`bDoFullDamage` true)
  (`GameplayStatics.SpawnEmitterAtLocation` "/Engine/Tutorial/SubEditors/TutorialAssets/TutorialParticleSystem.TutorialParticleSystem" _returnvalue)
  (`self.K2_DestroyActor`))

(fn `UserConstructionScript`)