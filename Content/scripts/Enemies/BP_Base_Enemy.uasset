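; Base enemy that scales health and walk speed with the game state's level and chases BP_MyCharacter.
; Tick either triggers a cooldown-gated Attack in range, flagging the material and damaging BP_TempCharacter, or runs AI MoveTo, jumping when a failed move's forward trace hits.
; Any and radial damage route through Punch, which updates a game-state stats meter and, on death, usually drops a randomly typed weapon.
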(event `self.ReceiveBeginPlay`
  (bind _newparam (message `/Game/scripts/Core/BI_BaseGameState.GetGaymLevelle` (`GameplayStatics.GetGameState`)))
  (set `self.health` (+ (`self.maxHealth`) _newparam))
  (set `CharacterMovementComponent.MaxWalkSpeed` (+ 800.0 (* (- _newparam 1) 50)) (`self.CharacterMovement`)))

(event `self.ReceiveTick`
  (params (DeltaSeconds :type "Float (single-precision)"))
  (bind _returnvalue (`self.K2_GetActorLocation`))
  (bind _returnvalue_2 (`GameplayStatics.GetActorOfClass` "/Game/scripts/Controller/BP_MyCharacter.BP_MyCharacter_C"))
  (if (< (`self.GetDistanceTo` _returnvalue_2) (`self.attackRange`))
    (if (`self.canAttack`)
      (`self.Attack`)
      (set `self.canAttack` false)
      (`KismetSystemLibrary.Delay` 1.0)
      (set `self.canAttack` true)
      (`MeshComponent.SetScalarParameterValueOnMaterials` (`self.Render`) "IsShoot" 0.0))
    (else
      (`KismetSystemLibrary.K2_SetTimerDelegate` :`Time` 0.5 :`bLooping` true)
      (`|AIMoveTo` self (`NavigationSystemV1.K2_ProjectPointToNavigation` (`self.K2_GetActorLocation` _returnvalue_2)) null 150.0
        (:`OnFail`
          (bind (_outhit _returnvalue_3) (`KismetSystemLibrary.SphereTraceSingle` _returnvalue (+ _returnvalue (* (`self.GetActorForwardVector`) 250.0)) 20.0 "TraceTypeQuery1"))
          (if _returnvalue_3
            (`self.Jump`)))))))

(event `/Game/scripts/Enemies/BI_Enemy.Punch`
  (params (damage :type "Float (double-precision)") (PunchDir :type "Vector Structure") (Type :type "EWeaponType Enum" :default "Melee"))
  (bind _returnvalue (- (`self.health`) damage))
  (if (`|EnumEquality` Type "Melee")
    (`GameplayStatics.PlaySound2D` "/Game/audio/StabCue.StabCue" 1.0 1.0 0.0 null null))
  (message `/Game/scripts/Core/BI_BaseGameState.AddStatsMeter` (`GameplayStatics.GetGameState`) 0.1)
  (`KismetSystemLibrary.PrintText` (`|FormatText` "remaining health:{X}" _returnvalue))
  (if (<= _returnvalue 0.0)
    (if (> (`KismetMathLibrary.RandomFloatInRange` 0.0 1.0) 0.2)
      (`|SpawnActorFromClass` "/Game/scripts/Weapons/BP_BaseWeapon.BP_BaseWeapon_C" (`self.GetTransform`) "Undefined" "MultiplyWithRoot" null (`KismetMathLibrary.SelectInt` 2 (`KismetMathLibrary.SelectInt` 1 0 (<= (`KismetMathLibrary.RandomFloatInRange` 0.0 1.0) 0.5)) (<= (`KismetMathLibrary.RandomFloatInRange` 0.0 1.0) 0.5)) null))
    (`self.K2_DestroyActor`)
    (else
      (set `self.health` _returnvalue))))

(event `self.ReceiveAnyDamage`
  (params (Damage :type "Float (single-precision)") (DamageType :type "DamageType Object Reference") (InstigatedBy :type "Controller Object Reference") (DamageCauser :type "Actor Object Reference"))
  (`self.Punch` Damage))

(event `self.ReceiveRadialDamage`
  (params (DamageReceived :type "Float (single-precision)") (DamageType :type "DamageType Object Reference") (Origin :type "Vector Structure") (HitInfo :type "HitResult Structure (by ref)") (InstigatedBy :type "Controller Object Reference") (DamageCauser :type "Actor Object Reference"))
  (`self.Punch` DamageReceived))

(fn `Attack`
  (`GameplayStatics.PlaySound2D` (`self.shootingCue`) 1.0 1.0 0.0 null null)
  (`MeshComponent.SetScalarParameterValueOnMaterials` (`self.Render`) "IsShoot" 1.0)
  (bind _returnvalue (`GameplayStatics.GetActorOfClass` "/Game/scripts/Core/BP_TempCharacter.BP_TempCharacter_C"))
  (`GameplayStatics.ApplyDamage` _returnvalue (`self.damage`)))

(fn `UserConstructionScript`)