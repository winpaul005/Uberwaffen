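; BP_BaseWeapon is a sprite pickup actor that serves as a medkit, ammo or weapon, depending on its Type.
; On BeginPlay it sets its sprite, rolling weapons from the Weapons data table, with RPG only possible when the GameState's died-too-much flag is set.
; Overlap by BP_TempCharacter heals, adds ammo or bags the weapon, then plays a sound and destroys the pickup.
; Each tick it billboards toward the player pawn.
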(event `self.ReceiveBeginPlay`
  (bind _papersprite (`self.PaperSprite`))
  (switch `int` (`self.Type`)
    (:`0`
      (`PaperSpriteComponent.SetSprite` _papersprite "/Game/sprites/s_medkit.s_medkit"))
    (:`1`
      (`PaperSpriteComponent.SetSprite` _papersprite "/Game/sprites/S_ammo.S_ammo"))
    (:`2`
      (bind _newparam (message `/Game/scripts/Core/BI_BaseGameState.GetHasDiedTooMuch` (`GameplayStatics.GetGameState`)))
      (bind _returnvalue (`|GetDataTableRow` "/Game/Weapons.Weapons" (`|GetArrayItem` (`|MakeArray` "KA420" "M82" "RPG" :!type "Name") (`KismetMathLibrary.RandomIntegerInRange` 0 (`KismetMathLibrary.SelectInt` 2 1 _newparam))))
        (:`then`
          (bind _output_get (set `self.weaponTyp` _returnvalue))
          (`PaperSpriteComponent.SetSprite` _papersprite (`.ItemImage` (break `WeaponItem` _output_get))))))))

(event `self.Box.OnComponentBeginOverlap`
  (params (OverlappedComponent :type "PrimitiveComponent Object Reference") (OtherActor :type "Actor Object Reference") (OtherComp :type "PrimitiveComponent Object Reference") (OtherBodyIndex :type Integer) (bFromSweep :type Boolean) (SweepResult :type "HitResult Structure (by ref)"))
  (bind _asbp_temp_character (cast `/Game/scripts/Core/BP_TempCharacter` OtherActor))
  (switch `int` (`self.Type`)
    (:`0`
      (`/Game/scripts/Core/BP_TempCharacter.Heal` _asbp_temp_character 15.0))
    (:`1`
      (`/Game/scripts/Core/BP_TempCharacter.AddAmmo` _asbp_temp_character))
    (:`2`
      (`/Game/scripts/Core/BP_TempCharacter.AddWeaponToBag` _asbp_temp_character (`self.weaponTyp`))))
  (`GameplayStatics.PlaySound2D` "/Game/audio/item_pickup.item_pickup" 1.0 1.0 0.0 null null)
  (`self.K2_DestroyActor`))

(event `self.ReceiveTick`
  (params (DeltaSeconds :type "Float (single-precision)"))
  (`SceneComponent.K2_SetWorldRotation` (`self.DefaultSceneRoot`) (`KismetMathLibrary.FindLookAtRotation` (`self.K2_GetActorLocation`) (`self.K2_GetActorLocation` (`GameplayStatics.GetPlayerPawn` 0))) false false))

(fn `UserConstructionScript`)