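; Temporary player character that carries a bag of weapons, switching and firing them through Enhanced Input, with damage stubbed as debug prints.
; BeginPlay fills the bag from three Weapons data table rows, and switching wraps through it, updating the mesh and GameState messages.
; The ProcessShot macro fires single shots on click, or full-auto on hold using a delta-time warmup/cooldown timer.
; Shoote spends ammo, exempts melee from the ammo check and calls the shoot event.
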(event `self.ReceiveBeginPlay`
  (`EnhancedInputSubsystemInterface.AddMappingContext` (pcsubsystem `EnhancedInputLocalPlayerSubsystem` (`GameplayStatics.GetPlayerController` 0)) "/Game/Inner/Maps/temp/IMC_TMP.IMC_TMP" 0 (struct))
  (bind _returnvalue (`|GetDataTableRow` "/Game/Weapons.Weapons" "KOMAROV")
    (:`then`
      (`self.AddWeaponToBag` _returnvalue)
      (bind _returnvalue_2 (`|GetDataTableRow` "/Game/Weapons.Weapons" "Shard")
        (:`then`
          (`self.AddWeaponToBag` _returnvalue_2)
          (bind _returnvalue_3 (`|GetDataTableRow` "/Game/Weapons.Weapons" "KA420")
            (:`then`
              (`self.AddWeaponToBag` _returnvalue_3))))))))

(event `EnhancedInput|/Game/Inner/Maps/temp/IA_Switch`
  (params (ActionValue :type "Float (double-precision)") (ElapsedSeconds :type "Float (double-precision)") (TriggeredSeconds :type "Float (double-precision)") (InputAction :type "InputAction Object Reference" :default "/Game/Inner/Maps/temp/IA_Switch.IA_Switch"))
  (:`Started`
    (if (< ActionValue 0.0)
      (`KismetSystemLibrary.PrintString` "Ping!")
      (`self.SwitchWep` true)
      (else
        (`KismetSystemLibrary.PrintString` "Pong!")
        (`self.SwitchWep` false)))))

(event `EnhancedInput|/Game/Inner/Maps/temp/IA_Shoot`
  (params (ActionValue :type Boolean) (ElapsedSeconds :type "Float (double-precision)") (TriggeredSeconds :type "Float (double-precision)") (InputAction :type "InputAction Object Reference" :default "/Game/Inner/Maps/temp/IA_Shoot.IA_Shoot"))
  (:`Triggered`
    (`self.ProcessShot` :!label _label))
  (:`Started`
    (goto _label :!via `Click`))
  (:`Completed`
    (`self.ShootEvent` true)
    (goto _label :!via `Release`)))

(fn `AddWeaponToBag`
  (params (NewItem :type "WeaponItem Structure (by ref)"))
  (bind _structout (setmembers `WeaponItem` :`StructRef` NewItem :`currentAmmo` (`.MaxAmmo` (break `WeaponItem` NewItem))))
  (bind _returnvalue (`KismetArrayLibrary.Array_Add` (`self.WeaponBag`) _structout))
  (set `self.CurrentWeapom` _returnvalue)
  (`self.UpdateVisuals` false))

(fn `Shoote`
  (bind _output (`|GetArrayItem` (`self.WeaponBag`) (`self.CurrentWeapom`)))
  (bind (_itemname _itemdescription _itemimage _viewportmesh _damagepattern _weapontype _maxammo _currentammo) (break `WeaponItem` _output))
  (if (or (> _currentammo 0) (`|EnumEquality` _weapontype "Melee"))
    (setmembers `WeaponItem` :`StructRef` _output :`currentAmmo` (`KismetMathLibrary.Clamp` (- _currentammo 1) 0 _maxammo))
    (switch `EWeaponType` _weapontype
      (:`Melee`
        (`KismetSystemLibrary.PrintString` "Damage Short"))
      (:`Ranged`
        (`KismetSystemLibrary.PrintString` "Damage long"))
      (:`Disposable`
        (`KismetSystemLibrary.PrintString` "Догони меня кирпич")))
    (`self.UpdateVisuals` true)
    (`self.ShootEvent` false)
    (else
      (`self.ShootEvent` true))))

(fn `SwitchWep`
  (params (IsReverse :type Boolean))
  (bind _currentweapom (`self.CurrentWeapom`))
  (bind _returnvalue (`KismetArrayLibrary.Array_Length` (`self.WeaponBag`)))
  (bind _returnvalue_2 (- _currentweapom 1))
  (bind _returnvalue_3 (+ _currentweapom 1))
  (if IsReverse
    (set `self.CurrentWeapom` (`KismetMathLibrary.SelectInt` (- _returnvalue 1) _returnvalue_2 (< _returnvalue_2 0)))
    (else
      (set `self.CurrentWeapom` (`KismetMathLibrary.SelectInt` 0 _returnvalue_3 (>= _returnvalue_3 _returnvalue)))))
  (`self.UpdateVisuals` false))

(fn `UpdateVisuals`
  (params (IsAmmo :type Boolean))
  (bind _returnvalue (`GameplayStatics.GetGameState`))
  (bind _output (`|GetArrayItem` (`self.WeaponBag`) (`self.CurrentWeapom`)))
  (bind (_itemname _itemdescription _itemimage _viewportmesh _damagepattern _weapontype _maxammo _currentammo) (break `WeaponItem` _output))
  (if IsAmmo
    (message `/Game/Inner/Maps/temp/BI_BaseGameState.UpdateAmmo` _returnvalue _currentammo _maxammo)
    (else
      (message `/Game/Inner/Maps/temp/BI_BaseGameState.UpdateWeapon` _returnvalue _output)
      (`SkeletalMeshComponent.SetSkeletalMeshAsset` (`self.Weapon`) _viewportmesh))))

(fn `UserConstructionScript`)